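; Area_C is a pressure-button trigger area that changes sky and music while the ThirdPersonCharacter stands in it.
; Capsule overlap speeds up SkyObj's clouds via RefreshMaterial, starts a 2D background cue, then briefly delays and nudges the actor down to look pressed.
; Leaving slows the clouds, stops the stored sound and, after a short delay, moves the actor to OriginalPosition.
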(event `self.Capsule.OnComponentBeginOverlap`
  (params (OverlappedComponent :type "PrimitiveComponent Object Reference") (OtherActor :type "Actor Object Reference") (OtherComp :type "PrimitiveComponent Object Reference") (OtherBodyIndex :type Integer) (bFromSweep :type Boolean) (SweepResult :type "HitResult Structure (by ref)"))
  (bind _skyobj (`self.SkyObj`))
  ;[1 1 1] When the player enters the area, play music, make the clouds turn faster, and make the button pressed
  (cast `/Game/ThirdPersonBP/Blueprints/ThirdPersonCharacter` OtherActor)
  (set `/Engine/EngineSky/BP_Sky_Sphere.Cloud speed` 1000.0 _skyobj)
  (`/Engine/EngineSky/BP_Sky_Sphere.RefreshMaterial` _skyobj)
  (bind _returnvalue (`GameplayStatics.SpawnSound2D` "/Game/StarterContent/Audio/Starter_Background_Cue.Starter_Background_Cue" 1.0 1.0 0.0 null))
  (set `self.2DSound` _returnvalue)
  (`KismetSystemLibrary.Delay` 0.02)
  (`self.K2_SetActorLocation` (- (`self.K2_GetActorLocation`) (0.0 0.0 2.0))))

(event `self.Capsule.OnComponentEndOverlap`
  (params (OverlappedComponent :type "PrimitiveComponent Object Reference") (OtherActor :type "Actor Object Reference") (OtherComp :type "PrimitiveComponent Object Reference") (OtherBodyIndex :type Integer))
  (bind _skyobj (`self.SkyObj`))
  ;[1 1 1] When the player exits the area, revert everything back to original
  (cast `/Game/ThirdPersonBP/Blueprints/ThirdPersonCharacter` OtherActor)
  (set `/Engine/EngineSky/BP_Sky_Sphere.Cloud speed` 2.0 _skyobj)
  (`/Engine/EngineSky/BP_Sky_Sphere.RefreshMaterial` _skyobj)
  (`AudioComponent.Stop` (`self.2DSound`))
  (`KismetSystemLibrary.Delay` 0.2)
  (`self.K2_SetActorLocation` (`self.OriginalPosition`)))

(fn `UserConstructionScript`)
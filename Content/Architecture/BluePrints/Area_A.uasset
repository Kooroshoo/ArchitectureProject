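; Area_A is a trigger-zone Blueprint that switches lights, a god ray and music as the player enters and leaves its capsule.
; Capsule overlap events filter for ThirdPersonCharacter, then toggle the visibility of PointLight, GodRay and PurpleLight on both entry and exit.
; Entry spawns a 2D starter music cue and stores it so exit can stop it.
; Visibility is flipped rather than set, so the on/off state depends on the components' initial visibility.
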(event `self.Capsule.OnComponentBeginOverlap`
  (params (OverlappedComponent :type "PrimitiveComponent Object Reference") (OtherActor :type "Actor Object Reference") (OtherComp :type "PrimitiveComponent Object Reference") (OtherBodyIndex :type Integer) (bFromSweep :type Boolean) (SweepResult :type "HitResult Structure (by ref)"))
  ;[1 1 1] When Player enters the area, turn the light, beam, music On
  (cast `/Game/ThirdPersonBP/Blueprints/ThirdPersonCharacter` OtherActor)
  (`SceneComponent.ToggleVisibility` (`self.PointLight`) false)
  (`SceneComponent.ToggleVisibility` (`self.GodRay`) false)
  (bind _returnvalue (`GameplayStatics.SpawnSound2D` "/Game/StarterContent/Audio/Starter_Music_Cue.Starter_Music_Cue" 1.0 1.0 0.0 null))
  (set `self.2DSound` _returnvalue)
  (`SceneComponent.ToggleVisibility` (`self.PurpleLight`) false))

(event `self.Capsule.OnComponentEndOverlap`
  (params (OverlappedComponent :type "PrimitiveComponent Object Reference") (OtherActor :type "Actor Object Reference") (OtherComp :type "PrimitiveComponent Object Reference") (OtherBodyIndex :type Integer))
  ;[1 1 1] When Player Exits the area, turn the light, beam, music Off
  (cast `/Game/ThirdPersonBP/Blueprints/ThirdPersonCharacter` OtherActor)
  (`SceneComponent.ToggleVisibility` (`self.PointLight`) false)
  (`SceneComponent.ToggleVisibility` (`self.GodRay`) false)
  (`AudioComponent.Stop` (`self.2DSound`))
  (`SceneComponent.ToggleVisibility` (`self.PurpleLight`) false))

(fn `UserConstructionScript`)
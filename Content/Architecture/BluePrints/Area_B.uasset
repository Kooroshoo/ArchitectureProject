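; Area_B is an actor whose height grows while the player's ThirdPersonCharacter stands inside its capsule and drops back when the character leaves.
; Capsule overlap events toggle an InCircle flag.
; Tick reads that flag and steps a stored TextureScale vector by Speed and delta time, applying it as actor scale within upper and lower Z-scale limits.
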(event `self.Capsule.OnComponentBeginOverlap`
  (params (OverlappedComponent :type "PrimitiveComponent Object Reference") (OtherActor :type "Actor Object Reference") (OtherComp :type "PrimitiveComponent Object Reference") (OtherBodyIndex :type Integer) (bFromSweep :type Boolean) (SweepResult :type "HitResult Structure (by ref)"))
  (cast `/Game/ThirdPersonBP/Blueprints/ThirdPersonCharacter` OtherActor)
  (set `self.InCircle` true))

(event `self.Capsule.OnComponentEndOverlap`
  (params (OverlappedComponent :type "PrimitiveComponent Object Reference") (OtherActor :type "Actor Object Reference") (OtherComp :type "PrimitiveComponent Object Reference") (OtherBodyIndex :type Integer))
  (cast `/Game/ThirdPersonBP/Blueprints/ThirdPersonCharacter` OtherActor)
  (set `self.InCircle` false))

(event `self.ReceiveTick`
  (params (DeltaSeconds :type "Float (single-precision)"))
  (bind _texturescale (`self.TextureScale`))
  (bind _texturescale_2 (`self.TextureScale`))
  (bind _z (.z (`self.GetActorScale3D`)))
  (set `self.DeltaTime` DeltaSeconds)
  (if (`self.InCircle`)
    ;[1 1 1] If ((Height Less than 90cm) and (in circle)) => Increase Height
    (if (<= _z 30.0)
      (`self.SetActorScale3D` _texturescale_2)
      (set `self.TextureScale` (+ _texturescale_2 (* (`KismetMathLibrary.Conv_DoubleToVector` (`self.DeltaTime`)) (`self.Speed`)))))
    (else
      ;[1 1 1] if ((height bigger than 1.1cm) and (Not in circle)) => Lower Height
      (if (>= _z 1.1)
        (`self.SetActorScale3D` _texturescale)
        (set `self.TextureScale` (- _texturescale (* (`KismetMathLibrary.Conv_DoubleToVector` (`self.DeltaTime`)) (`self.Speed`))))))))

(fn `UserConstructionScript`)